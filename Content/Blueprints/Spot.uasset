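; Spot is a board position actor that spawns and configures a game piece for the selected level when play begins.
; BeginPlay loads the player save and the level design save, then spawns a Piece slightly above itself.
; The piece's material and mesh come from the clicked level's entry at this spot's Number, with random picks from color and shape lists when unset.
; A disconnected debug preview with text renders remains unused.
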(event `self.ReceiveBeginPlay`
  (bind _item (`KismetArrayLibrary.Array_Get` (`.Color_42_2D6E2024484AF4F4B5B830A207543E43` (break `/Game/Blueprints/S_LevelsLayout` (`KismetArrayLibrary.Array_Get` (`/Game/Blueprints/SG_LD.Level Design` (`self.C SG LD`)) (`/Game/Blueprints/SG_Save.Clicked Level` (`self.C_SG_Save`))))) (`self.Number`)))
  (bind _item_2 (`KismetArrayLibrary.Array_Get` (`.Shape_43_47D4A0DD4AE20067A95E218EFEADE2F3` (break `/Game/Blueprints/S_LevelsLayout` (`KismetArrayLibrary.Array_Get` (`/Game/Blueprints/SG_LD.Level Design` (`self.C SG LD`)) (`/Game/Blueprints/SG_Save.Clicked Level` (`self.C_SG_Save`))))) (`self.Number`)))
  (`|ExecutionSequence`
    (:`then_0`
      (`GameplayStatics.DoesSaveGameExist` "Save")
      (if true
        (bind _returnvalue (`GameplayStatics.LoadGameFromSlot` "Save"))
        (bind _assg_save (cast `/Game/Blueprints/SG_Save` _returnvalue))
        (set `self.C_SG_Save` _assg_save)))
    (:`then_1`
      (bind _returnvalue_2 (`GameplayStatics.DoesSaveGameExist` (`self.LevelDesignLocation`)))
      (if _returnvalue_2
        (bind _returnvalue_3 (`GameplayStatics.LoadGameFromSlot` (`self.LevelDesignLocation`)))
        (bind _assg_ld (cast `/Game/Blueprints/SG_LD` _returnvalue_3))
        (set `self.C SG LD` _assg_ld)))
    (:`then_2`
      (bind _returnvalue_4 (`|SpawnActorFromClass` "/Game/Blueprints/Piece.Piece_C" (`KismetMathLibrary.MakeTransform` (`KismetMathLibrary.MakeVector` (.x (.location (`SceneComponent.K2_GetComponentToWorld` (`self.Spot`)))) (.y (.location (`SceneComponent.K2_GetComponentToWorld` (`self.Spot`)))) (+ (.z (.location (`SceneComponent.K2_GetComponentToWorld` (`self.Spot`)))) 10.0)) (.rotation (`SceneComponent.K2_GetComponentToWorld` (`self.Spot`))) (.scale (`SceneComponent.K2_GetComponentToWorld` (`self.Spot`)))) "AlwaysSpawn" "OverrideRootScale"))
      (set `self.Piece` _returnvalue_4)
      ;[1 1 1] Set Material Information
      (`/Engine/EditorBlueprintResources/StandardMacros.IsValid` _item
        (:`Is Valid`
          (set `self.Color` _item))
        (:`Is Not Valid`
          (set `self.Color` (`KismetArrayLibrary.Array_Get` (`self.Colors List`) (`KismetMathLibrary.RandomIntegerInRange` 0 (`KismetArrayLibrary.Array_LastIndex` (`self.Colors List`)))))))
      (set `self.Color Text` (`KismetTextLibrary.Conv_ObjectToText` (`self.Color`)))
      (`PrimitiveComponent.SetMaterial` (`/Game/Blueprints/Piece.Piece` (`self.Piece`)) 0 (`self.Color`))
      (set `/Game/Blueprints/Piece.Color Text` (`self.Color Text`) (`self.Piece`))
      ;[1 1 1] Set Shape Information
      (`/Engine/EditorBlueprintResources/StandardMacros.IsValid` _item_2
        (:`Is Valid`
          (set `self.Shape` _item_2))
        (:`Is Not Valid`
          (set `self.Shape` (`KismetArrayLibrary.Array_Get` (`self.Shapes List`) (`KismetMathLibrary.RandomIntegerInRange` 0 (`KismetArrayLibrary.Array_LastIndex` (`self.Shapes List`)))))))
      (set `self.Shape Text` (`KismetTextLibrary.Conv_ObjectToText` (`self.Shape`)))
      (`StaticMeshComponent.SetStaticMesh` (`/Game/Blueprints/Piece.Piece` (`self.Piece`)) (`self.Shape`))
      (set `/Game/Blueprints/Piece.Shape Text` (`self.Shape Text`) (`self.Piece`))
      (`SceneComponent.SetWorldScale3D` (`/Game/Blueprints/Piece.Piece` (`self.Piece`)) (0.6 0.6 0.6))
      (set `/Game/Blueprints/Piece.Number` (`self.Number`) (`self.Piece`)))))

(fn `UserConstructionScript`)