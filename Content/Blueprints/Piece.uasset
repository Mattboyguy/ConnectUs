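; A numbered grid puzzle piece that picks its icon from its color and shape on BeginPlay, with Plus shapes reusing the Square icons.
; DropDown sphere-traces along -X to count spots and pieces below, then eases the piece down over the empty spots.
; It then traces downward in Z to copy the underlying Spot's number to its label.
; Cosmetic events start and stop a Hover timeline that scales the piece.
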(event `self.ReceiveBeginPlay`
  (`TextRenderComponent.K2_SetText` (`self.Number Render`) (`KismetTextLibrary.Conv_IntToText` (`self.Number`)))
  (switch `string` (`KismetStringLibrary.Concat_StrStr` (`KismetTextLibrary.Conv_TextToString` (`self.Color Text`)) " " (`KismetTextLibrary.Conv_TextToString` (`self.Shape Text`)))
    (:`Blue Triangle`
      (set `self.Icon` "/Game/Images/Triange_Blue.Triange_Blue"))
    (:`Red Triangle`
      (set `self.Icon` "/Game/Images/Triangle_Red.Triangle_Red"))
    (:`Green Triangle`
      (set `self.Icon` "/Game/Images/Triangle_Green.Triangle_Green"))
    (:`Orange Triangle`
      (set `self.Icon` "/Game/Images/Triangle_Orange.Triangle_Orange"))
    (:`Blue Circle`
      (set `self.Icon` "/Game/Images/Circle_Blue.Circle_Blue"))
    (:`Red Circle`
      (set `self.Icon` "/Game/Images/Circle_Red.Circle_Red"))
    (:`Green Circle`
      (set `self.Icon` "/Game/Images/Circle_Green.Circle_Green"))
    (:`Orange Circle`
      (set `self.Icon` "/Game/Images/Circle_Orange.Circle_Orange"))
    (:`Blue Square`
      (set `self.Icon` "/Game/Images/Square_Blue.Square_Blue"))
    (:`Red Square`
      (set `self.Icon` "/Game/Images/Square_Red.Square_Red"))
    (:`Green Square`
      (set `self.Icon` "/Game/Images/Square_Green.Square_Green"))
    (:`Orange Square`
      (set `self.Icon` "/Game/Images/Square_Orange.Square_Orange"))
    (:`Blue Plus`
      (set `self.Icon` "/Game/Images/Square_Blue.Square_Blue"))
    (:`Red Plus`
      (set `self.Icon` "/Game/Images/Square_Red.Square_Red"))
    (:`Green Plus`
      (set `self.Icon` "/Game/Images/Square_Green.Square_Green"))
    (:`Orange Plus`
      (set `self.Icon` "/Game/Images/Square_Orange.Square_Orange"))))

(event `Drop Down`
  (bind (_returnvalue_x _returnvalue_y _returnvalue_z) (`KismetMathLibrary.BreakVector` (`self.K2_GetActorLocation`)))
  (bind (_returnvalue_x_2 _returnvalue_y_2 _returnvalue_z_2) (`KismetMathLibrary.BreakVector` (`self.K2_GetActorLocation`)))
  (bind (_returnvalue_x_3 _returnvalue_y_3 _returnvalue_z_3) (`KismetMathLibrary.BreakVector` (`self.K2_GetActorLocation`)))
  (bind (_returnvalue_x_4 _returnvalue_y_4 _returnvalue_z_4) (`KismetMathLibrary.BreakVector` (`self.K2_GetActorLocation`)))
  (bind _outhits (`KismetSystemLibrary.SphereTraceMultiForObjects` (`self.K2_GetActorLocation`) (`KismetMathLibrary.MakeVector` (- _returnvalue_x_3 10000.0) _returnvalue_y_3 _returnvalue_z_3) 50.0 (`|MakeArray` "ObjectTypeQuery7" :!type "EObjectTypeQuery Enum")))
  (set `self.Spots Below` (`KismetArrayLibrary.Array_LastIndex` _outhits))
  (bind _outhits_2 (`KismetSystemLibrary.SphereTraceMultiForObjects` (`self.K2_GetActorLocation`) (`KismetMathLibrary.MakeVector` (- _returnvalue_x 10000.0) _returnvalue_y _returnvalue_z) 50.0 (`|MakeArray` "ObjectTypeQuery8" :!type "EObjectTypeQuery Enum")))
  (set `self.Pieces Below` (`KismetArrayLibrary.Array_Length` _outhits_2))
  (`KismetSystemLibrary.MoveComponentTo` (`self.Scene`) (`KismetMathLibrary.MakeVector` (+ (* (- (`self.Spots Below`) (`self.Pieces Below`)) -200.0) _returnvalue_x_4) _returnvalue_y_4 _returnvalue_z_4) (`SceneComponent.K2_GetComponentRotation` (`self.Scene`)) true false 0.2)
  ;[1 1 1] Change Number on Piece to Spot Number
  (bind _outhit (`KismetSystemLibrary.SphereTraceSingleForObjects` (`self.K2_GetActorLocation`) (`KismetMathLibrary.MakeVector` _returnvalue_x_2 _returnvalue_y_2 (- _returnvalue_z_2 50.0)) 25.0 (`|MakeArray` "ObjectTypeQuery7" :!type "EObjectTypeQuery Enum")))
  (bind _asspot (cast `/Game/Blueprints/Spot` (`.HitActor` (`GameplayStatics.BreakHitResult` _outhit))))
  (bind _output_get (set `self.Number` (`/Game/Blueprints/Spot.Number` _asspot)))
  (`TextRenderComponent.K2_SetText` (`self.Number Render`) (`KismetTextLibrary.Conv_IntToText` _output_get)))

(event `Cosmetic Effect - Play`
  (bind (_direction _scale) (`Timeline|Hover` :!via `PlayFromStart` :!label _label)
    (:`Update`
      (`SceneComponent.SetWorldScale3D` (`self.Piece`) (`KismetMathLibrary.MakeVector` _scale _scale 0.5)))))

(event `Cosmetic Event - Stop`
  (goto _label :!via `Stop`))

(fn `UserConstructionScript`)