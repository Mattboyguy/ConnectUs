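; Game instance Blueprint holding an empty GooglePlayLogin event and a disconnected Google Play sign-in and in-app purchase flow.
; The unwired chain would show the external login UI, query two product IDs on success, and copy the results into IAPArray on itself and the PC_Menu player controller.
; Print strings mark each outcome, but none of this runs because no event leads into it.
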(event `Google Play Login`)