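; TopSpot is a numbered spawn point that creates game pieces with a random color and shape.
; At BeginPlay it spawns a hidden Piece just above its Spot, assigning a random material and mesh and copying their names and the spot's Number onto it.
; AddPiece and CheckforPiece use sphere traces to spawn another piece only when nothing is hit.
; The construction script displays the Number on its text component.
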(event `Add Piece`
  (bind (_start _end) (`self.Start and End` -200.0))
  (bind (_outhit _returnvalue) (`KismetSystemLibrary.SphereTraceSingle_NEW` _start _end 25.0 "TraceTypeQuery1"))
  (if (not _returnvalue)
    (`self.Create New Piece`)))

(event `Create New Piece`
  (bind _returnvalue (`|SpawnActorFromClass` "/Game/Blueprints/Piece.Piece_C" (`KismetMathLibrary.MakeTransform` (`KismetMathLibrary.MakeVector` (.x (.location (`SceneComponent.K2_GetComponentToWorld` (`self.Spot`)))) (.y (.location (`SceneComponent.K2_GetComponentToWorld` (`self.Spot`)))) (+ (.z (.location (`SceneComponent.K2_GetComponentToWorld` (`self.Spot`)))) 10.0)) (.rotation (`SceneComponent.K2_GetComponentToWorld` (`self.Spot`))) (.scale (`SceneComponent.K2_GetComponentToWorld` (`self.Spot`)))) "Undefined" "OverrideRootScale" :!label _label))
  (set `self.Piece` _returnvalue)
  ;[1 1 1] Set Material Information
  (set `self.Color` (`KismetArrayLibrary.Array_Get` (`self.Colors List`) (`KismetMathLibrary.RandomIntegerInRange` 0 (`KismetArrayLibrary.Array_LastIndex` (`self.Colors List`)))))
  (set `self.Color Text` (`KismetTextLibrary.Conv_ObjectToText` (`self.Color`)))
  (`PrimitiveComponent.SetMaterial` (`/Game/Blueprints/Piece.Piece` (`self.Piece`)) 0 (`self.Color`))
  (set `/Game/Blueprints/Piece.Color Text` (`self.Color Text`) (`self.Piece`))
  ;[1 1 1] Set Shape Information
  (set `self.Shape` (`KismetArrayLibrary.Array_Get` (`self.Shapes List`) (`KismetMathLibrary.RandomIntegerInRange` 0 (`KismetArrayLibrary.Array_LastIndex` (`self.Shapes List`)))))
  (set `self.Shape Text` (`KismetTextLibrary.Conv_ObjectToText` (`self.Shape`)))
  (`StaticMeshComponent.SetStaticMesh` (`/Game/Blueprints/Piece.Piece` (`self.Piece`)) (`self.Shape`))
  (set `/Game/Blueprints/Piece.Shape Text` (`self.Shape Text`) (`self.Piece`))
  (`SceneComponent.SetWorldScale3D` (`/Game/Blueprints/Piece.Piece` (`self.Piece`)) (0.6 0.6 0.6))
  (set `/Game/Blueprints/Piece.Number` (`self.Number`) (`self.Piece`))
  (`self.SetActorHiddenInGame` (`self.Piece`) true))

(event `self.ReceiveBeginPlay`
  (goto _label))

(event `Check for Piece`
  (bind (_returnvalue_x _returnvalue_y _returnvalue_z) (`KismetMathLibrary.BreakVector` (`self.K2_GetActorLocation`)))
  (bind (_outhit _returnvalue) (`KismetSystemLibrary.SphereTraceSingleForObjects` (`self.K2_GetActorLocation`) (`KismetMathLibrary.MakeVector` _returnvalue_x _returnvalue_y (- _returnvalue_z -50.0)) 25.0 (`|MakeArray` "ObjectTypeQuery8" :!type "EObjectTypeQuery Enum")))
  (if (not _returnvalue)
    (`self.Create New Piece`)))

(fn `UserConstructionScript`
  (`TextRenderComponent.K2_SetText` (`self.Number Text`) (`KismetTextLibrary.Conv_IntToText` (`self.Number`))))