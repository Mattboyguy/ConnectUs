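; Spline actor that builds spline mesh segments between consecutive points of its Spline through the custom AddSplineEvent.
; UpdateSpline re-enters the shared SetStartAndEnd step without creating components, so it only reaches the last one added.
; That step reads UpdateSpline's loop index, even when run from AddSplineEvent.
; The construction script does nothing; a similar segment-building loop there is disconnected.
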(event `Add Spline Event`
  (bind _spline (`self.Spline`))
  (for _ (range (+ (- (`SplineComponent.GetNumberOfSplinePoints` (`self.Spline`)) 2) 1))
    (bind _returnvalue (`AddComponent|NODE_AddSplineMeshComponent-3`))
    (`SceneComponent.K2_AttachToComponent` _returnvalue null "None" "KeepWorld" "KeepWorld" "KeepWorld" false)
    (bind (_location _tangent) (`SplineComponent.GetLocationAndTangentAtSplinePoint` _spline (stale `Update Spline` _index) "Local"))
    (bind (_location_2 _tangent_2) (`SplineComponent.GetLocationAndTangentAtSplinePoint` _spline (+ (stale `Update Spline` _index) 1) "Local"))
    (`SplineMeshComponent.SetStartAndEnd` _returnvalue _location _tangent _location_2 _tangent_2 true :!label _label)))

(event `Update Spline`
  (for _index (range (+ (- (`SplineComponent.GetNumberOfSplinePoints` (`self.Spline`)) 2) 1))
    (goto _label)))

(fn `UserConstructionScript`)