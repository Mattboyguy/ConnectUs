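; Menu pawn whose only active logic is a 1-key shortcut that empties the player's saved lives.
; The key press loads the "Save" slot as SG_Save, zeroes Lives, stamps LifeTimer with the current real-time seconds and saves it back.
; It then finds HUD_Menu by class, swaps the full-lives display for the timer, reruns InitiateStartup and removes all W_Lives widgets.
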(event `Key|One`
  (params (Key :type "Key Structure" :default "AnyKey"))
  (:`Pressed`
    (bind _returnvalue (`GameplayStatics.LoadGameFromSlot` "Save"))
    (bind _assg_save (cast `/Game/Blueprints/SG_Save` _returnvalue))
    (set `/Game/Blueprints/SG_Save.Lives` 0 _assg_save)
    (set `/Game/Blueprints/SG_Save.LifeTimer` (`GameplayStatics.GetAccurateRealTime`) _assg_save)
    (`GameplayStatics.SaveGameToSlot` _assg_save "Save")
    (bind _foundwidgets (`WidgetBlueprintLibrary.GetAllWidgetsOfClass` "/Game/Blueprints/MainMenu/HUD_Menu.HUD_Menu_C"))
    (bind _item (`KismetArrayLibrary.Array_Get` _foundwidgets))
    (`Widget.SetVisibility` (`/Game/Blueprints/MainMenu/HUD_Menu.LifeTimer` _item) "Visible")
    (`Widget.SetVisibility` (`/Game/Blueprints/MainMenu/HUD_Menu.FullLives` _item) "Collapsed")
    (`/Game/Blueprints/MainMenu/HUD_Menu.Initiate Startup` _item)
    (bind _foundwidgets_2 (`WidgetBlueprintLibrary.GetAllWidgetsOfClass` "/Game/Blueprints/MainMenu/W_Lives.W_Lives_C" false))
    (for _array_element _foundwidgets_2
      (`Widget.RemoveFromParent` _array_element))))

(fn `UserConstructionScript`)