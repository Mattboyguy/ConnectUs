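; Menu player controller that brings up the main menu HUD and prepares save data and in-app purchases on BeginPlay.
; It creates the HUD_Menu widget with game-and-UI input, creates missing Save and Stats slots, and calls InitiateStartup on the HUD when Save was absent.
; It then queries IAP products, showing the external login UI first if needed, and passes results to each market tile widget.
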(event `self.ReceiveBeginPlay`
  (`|ExecutionSequence`
    (:`then_0`
      (bind _returnvalue (`|CreateWidget` "/Game/Blueprints/MainMenu/HUD_Menu.HUD_Menu_C"))
      (bind _output_get (set `self.C_Menu_HUD` _returnvalue))
      (`UserWidget.AddToViewport` _output_get 0)
      (`WidgetBlueprintLibrary.SetInputMode_GameAndUIEx` (`GameplayStatics.GetPlayerController` 0) null "DoNotLock" false))
    (:`then_1`
      (bind _returnvalue_2 (`GameplayStatics.DoesSaveGameExist` "Save"))
      (if (not _returnvalue_2)
        (bind _returnvalue_3 (`GameplayStatics.CreateSaveGameObject` "/Game/Blueprints/SG_Save.SG_Save_C"))
        (bind _output_get_2 (set `self.C_SG_Save` _returnvalue_3))
        (`GameplayStatics.SaveGameToSlot` _output_get_2 "Save")
        (bind _foundwidgets (`WidgetBlueprintLibrary.GetAllWidgetsOfClass` "/Game/Blueprints/MainMenu/HUD_Menu.HUD_Menu_C"))
        (`/Game/Blueprints/MainMenu/HUD_Menu.Initiate Startup` (`KismetArrayLibrary.Array_Get` _foundwidgets))))
    (:`then_2`
      (bind _returnvalue_4 (`GameplayStatics.DoesSaveGameExist` "Stats"))
      (if (not _returnvalue_4)
        (bind _returnvalue_5 (`GameplayStatics.CreateSaveGameObject` "/Game/Blueprints/SG_Stats.SG_Stats_C"))
        (`GameplayStatics.SaveGameToSlot` _returnvalue_5 "Stats")))
    (:`then_3`
      (if (`KismetSystemLibrary.IsLoggedIn` (`GameplayStatics.GetPlayerController` 0))
        (bind _inapppurchaseinformation (`|InAppPurchaseQuery` (`GameplayStatics.GetPlayerController` 0) (`|MakeArray` "0001_iap" "0002_iap" "0003_iap" "0004_iap") :!label _label)
          (:`OnSuccess`
            (`KismetSystemLibrary.PrintString` "Loaded IAP")
            (bind _foundwidgets_2 (`WidgetBlueprintLibrary.GetAllWidgetsOfClass` "/Game/Blueprints/MainMenu/W_Market_Tile.W_Market_Tile_C" false))
            (set `self.IAP Array` _inapppurchaseinformation)
            (for _array_element _foundwidgets_2
              (`/Game/Blueprints/MainMenu/W_Market_Tile.Initiate IAP Data` _array_element _inapppurchaseinformation)))
          (:`OnFailure`
            (`KismetSystemLibrary.PrintString` "Failed to Load IAP")))
        (else
          (`ShowLoginUICallbackProxy.ShowExternalLoginUI` (`GameplayStatics.GetPlayerController` 0)
            (:`then`
              (set `self.Signing In` "Visible"))
            (:`OnSuccess`
              (set `self.Signing In` "Collapsed")
              (goto _label))))))))

(fn `UserConstructionScript`)